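; BP_Archer is the Archer NPC, which drives a talk prompt when another actor enters or leaves its Box trigger.
; Begin and end overlap call TalkPromtMessage on that actor to switch the prompt on or off, passing a fixed speaker ID, and store the result in Overlap.
; GetLocation returns the mesh's world position, and OverlapWithPlayer exposes the stored Overlap value.
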(event `self.Box.OnComponentBeginOverlap`
  (params (OverlappedComponent :type "PrimitiveComponent Object Reference") (OtherActor :type "Actor Object Reference") (OtherComp :type "PrimitiveComponent Object Reference") (OtherBodyIndex :type Integer) (bFromSweep :type Boolean) (SweepResult :type "HitResult Structure (by ref)"))
  (bind _overlap (message `/Game/FirstPerson/Blueprints/BPI_Player.TalkPromt` OtherActor true 3))
  (set `self.Overlap` _overlap))

(event `self.Box.OnComponentEndOverlap`
  (params (OverlappedComponent :type "PrimitiveComponent Object Reference") (OtherActor :type "Actor Object Reference") (OtherComp :type "PrimitiveComponent Object Reference") (OtherBodyIndex :type Integer))
  (bind _overlap (message `/Game/FirstPerson/Blueprints/BPI_Player.TalkPromt` OtherActor false 3))
  (set `self.Overlap` _overlap))

(fn `GetLocation`
  (returns (CurrentLocation :type "Vector Structure"))
  (return (`SceneComponent.K2_GetComponentLocation` (`self.Mesh`))))

(fn `OverlapWithPlayer`
  (returns (`HasPlayerOverlap?` :type Boolean))
  (return (`self.Overlap`)))

(fn `UserConstructionScript`)