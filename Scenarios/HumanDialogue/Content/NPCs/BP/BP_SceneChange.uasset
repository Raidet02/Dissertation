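; BP_SceneChange is a trigger actor that marks a spot where a scene change can be offered to an overlapping actor.
; While the change is available, its box overlap sends ChangeSceneMessage to that actor on enter and exit, passing an on/off flag and a self reference.
; SetChangeScene toggles that availability and shows or hides a point light to match.
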(event `self.Box.OnComponentBeginOverlap`
  (params (OverlappedComponent :type "PrimitiveComponent Object Reference") (OtherActor :type "Actor Object Reference") (OtherComp :type "PrimitiveComponent Object Reference") (OtherBodyIndex :type Integer) (bFromSweep :type Boolean) (SweepResult :type "HitResult Structure (by ref)"))
  (if (`self.ChangeAvalible?`)
    (message `/Game/FirstPerson/Blueprints/BPI_Player.ChangeScene` OtherActor true self)))

(event `self.Box.OnComponentEndOverlap`
  (params (OverlappedComponent :type "PrimitiveComponent Object Reference") (OtherActor :type "Actor Object Reference") (OtherComp :type "PrimitiveComponent Object Reference") (OtherBodyIndex :type Integer))
  (if (`self.ChangeAvalible?`)
    (message `/Game/FirstPerson/Blueprints/BPI_Player.ChangeScene` OtherActor false self)))

(event `/Game/NPCs/BP/BPI_SceneChange.SetChangeScene`
  (params (`ChangeAvalible?` :type Boolean))
  (bind _output_get (set `self.ChangeAvalible?` `ChangeAvalible?`))
  (if _output_get
    (`SceneComponent.SetVisibility` (`self.PointLight`) true false)
    (else
      (`SceneComponent.SetVisibility` (`self.PointLight`) false false))))

(fn `UserConstructionScript`)